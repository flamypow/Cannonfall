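; BP_Hazard is a hazard actor that kills the player on impact and ends the game.
; A Sphere hit on the player, or on anything while the player is inside GroundCollision, destroys all Player-tagged actors.
; After a brief delay it pauses the game and shows the game-over widget.
; A hit that misses the player destroys the hazard after a short delay.
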(event `self.Sphere.OnComponentHit`
  (params (HitComponent :type "PrimitiveComponent Object Reference") (OtherActor :type "Actor Object Reference") (OtherComp :type "PrimitiveComponent Object Reference") (NormalImpulse :type "Vector Structure") (Hit :type "HitResult Structure (by ref)"))
  (if (`self.ActorHasTag` OtherActor "Player")
    (bind _outactors (`GameplayStatics.GetAllActorsWithTag` "Player" :!label _label))
    (`self.K2_DestroyActor` _outactors)
    (`KismetSystemLibrary.Delay` 0.07)
    (`GameplayStatics.SetGamePaused` true)
    (bind _returnvalue (`|CreateWidget` "/Game/WilliamChen/Blueprints/BP_UI_GameOverWidget.BP_UI_GameOverWidget_C"))
    (`UserWidget.AddToViewport` _returnvalue 0)
    (elif (`self.IsPlayerInside`)
      (goto _label)
      (else
        _)))
  (`KismetSystemLibrary.Delay` 0.07)
  (`self.K2_DestroyActor`))

(event `self.GroundCollision.OnComponentBeginOverlap`
  (params (OverlappedComponent :type "PrimitiveComponent Object Reference") (OtherActor :type "Actor Object Reference") (OtherComp :type "PrimitiveComponent Object Reference") (OtherBodyIndex :type Integer) (bFromSweep :type Boolean) (SweepResult :type "HitResult Structure (by ref)"))
  (if (`self.ActorHasTag` OtherActor "Player")
    (set `self.IsPlayerInside` true)))

(event `self.GroundCollision.OnComponentEndOverlap`
  (params (OverlappedComponent :type "PrimitiveComponent Object Reference") (OtherActor :type "Actor Object Reference") (OtherComp :type "PrimitiveComponent Object Reference") (OtherBodyIndex :type Integer))
  (if (`self.ActorHasTag` OtherActor "Player")
    (set `self.IsPlayerInside` false)))

(fn `UserConstructionScript`)